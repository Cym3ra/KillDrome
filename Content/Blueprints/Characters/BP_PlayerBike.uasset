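; Player bike Blueprint that orients its mesh every tick from steering and terrain.
; Lean roll eases toward a clamped target built from speed and steering input.
; Line traces at the front and back wheel sockets then set the mesh's world rotation along the ground, overwriting the roll just applied.
; GetTurnAngle exposes the raw steering input.
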(event EventBeginPlay)

(event Collision|EventActorBeginOverlap
  (params (OtherActor :type Actor%20Object%20Reference)))

(event EventTick
  (params (DeltaSeconds :type Float%20%28single-precision%29))
  (CallFunction|UpdateLeanAngle)
  (|AlignVehicle))

(fn ConstructionScript)

(fn UpdateLeanAngle
  (Transformation|SetRelativeRotation (Variables|Character|GetMesh) (Math|Rotator|MakeRotator (Variables|Default|GetLeanAngle) 0.0 0.0) false false)
  (Variables|Default|SetLeanAngle (Math|Float|Lerp (Variables|Default|GetLeanAngle) (Math|Float|Clamp(Float) (* (/ (Math|Vector|VectorLength (Transformation|GetVelocity)) 2e+03) (* (Input|EnhancedActionValues|GetIA_Steering) 12.0)) -12.0 2e+01) 0.02)))

(fn WheelTrace
  (params (InputPin :type Vector))
  (bind (_outhit _returnvalue) (Collision|LineTraceByChannel (+ InputPin "0.000000,0.000000,100.000000") (+ InputPin "0.000000,0.000000,-100.000000") "TraceTypeQuery1" false 0 "None"))
  (if _returnvalue
    (return (.Location (Collision|BreakHitResult _outhit)))
    (else
      (return InputPin))))

(fn GetTurnAngle
  (return (Input|EnhancedActionValues|GetIA_Steering)))